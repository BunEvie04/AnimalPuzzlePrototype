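; AI controller for a Foxling animal that runs a behavior tree and keeps its survival data in the Blackboard.
; BeginPlay starts the tree and fills energy; Tick calls RunBehaviorTree again, writes the controller's own location and drains energy per frame, independent of delta time.
; Tick also looks up one BP_Grass actor, publishing its location and validity when visible, or flagging it invalid when hidden.
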(event EventTick
  (params (DeltaSeconds :type Float%20%28single-precision%29))
  (bind _keyenergy (Variables|Default|GetKeyEnergy))
  (bind _blackboard (Variables|Default|GetBlackboard))
  ;[1 1 1] Sets up animal variables in Blackboard
  (AI|RunBehaviorTree (Variables|Default|GetBTAsset))
  (AI|Components|Blackboard|SetValueasVector _blackboard (Variables|BlackBoard|GetKey%20Name%20Animal) (Transformation|GetActorLocation))
  ;[1 1 1] Removes energy every tick
  (AI|Components|Blackboard|SetValueasFloat _blackboard _keyenergy (- (Class|BlackboardComponent|GetValueasFloat _blackboard _keyenergy) 0.01))
  ;[1 1 1] Sets up Grass location
  (bind _returnvalue (Actor|GetActorOfClass "/Game/Dynamic/ItemMechanic/PrototypeItems/BP_Grass.BP_Grass_C"))
  (Utilities|IsValid _returnvalue
    (:Is%20Valid
      (if (Variables|/Script/Engine.Actor|GetbHidden _returnvalue)
        (AI|Components|Blackboard|SetValueasBool (Variables|Default|GetBlackboard) (Variables|BlackBoard|GetKey%20Valid) false)
        (else
          (AI|Components|Blackboard|SetValueasVector (Variables|Default|GetBlackboard) (Variables|BlackBoard|GetKey%20Name%20Grass) (Transformation|GetActorLocation _returnvalue))
          (AI|Components|Blackboard|SetValueasBool (Variables|Default|GetBlackboard) (Variables|BlackBoard|GetKey%20Valid) true))))))

(event EventBeginPlay
  ;[1 1 1] Runs Behaviour Tree
  (AI|RunBehaviorTree (Variables|Default|GetBTAsset))
  (AI|Components|Blackboard|SetValueasFloat (Variables|Default|GetBlackboard) (Variables|Default|GetKey%20Name%20Energy) 1e+02))

(fn ConstructionScript)