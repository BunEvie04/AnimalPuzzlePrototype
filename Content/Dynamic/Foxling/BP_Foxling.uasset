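; BP_Foxling is a Foxling character that exposes UpdateMovement to set its max walk speed.
; Its capsule overlap casts to BP_Platform and waits one second, with nothing after the delay.
; Disconnected leftovers hold a random-point AIMoveTo wander loop, a forward line trace, look-at rotation and a platform collision change, none of which run.
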(event OnComponentBeginOverlap(CapsuleComponent)
  (params (OverlappedComponent :type Primitive%20Component%20Object%20Reference) (OtherActor :type Actor%20Object%20Reference) (OtherComp :type Primitive%20Component%20Object%20Reference) (OtherBodyIndex :type Integer) (bFromSweep :type Boolean) (SweepResult :type Hit%20Result%20Structure%20%28by%20ref%29))
  (bind _asbp_platform (Utilities|Casting|CastToBP_Platform OtherActor))
  (Utilities|FlowControl|Delay 1.0))

(event Collision|EventActorBeginOverlap
  (params (OtherActor :type Actor%20Object%20Reference)))

(event EventTick
  (params (DeltaSeconds :type Float%20%28single-precision%29)))

(fn ConstructionScript)

(fn UpdateMovement
  (params (NewWalkSpeed :type Float%20%28double-precision%29))
  (Variables|/Script/Engine.CharacterMovementComponent|SetMaxWalkSpeed (Variables|Character|GetCharacterMovement) NewWalkSpeed))