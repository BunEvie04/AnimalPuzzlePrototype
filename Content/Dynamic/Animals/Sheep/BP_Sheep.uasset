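; Sheep animal that spots food and reacts to Kibby, playing one random sheep sound shortly after spawn.
; Pawn sensing looks up the seen class's name in the Fruit table, feeds eat time to the blackboard and notifies AC_Sheep.
; KibbySensor overlaps reverse a moving AutoSpline, with end overlap continuing it.
; Fire fleeing and hunger logic are left unconnected.
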(event OnComponentBeginOverlap(KibbySensor)
  (params (OverlappedComponent :type Primitive%20Component%20Object%20Reference) (OtherActor :type Actor%20Object%20Reference) (OtherComp :type Primitive%20Component%20Object%20Reference) (OtherBodyIndex :type Integer) (bFromSweep :type Boolean) (SweepResult :type Hit%20Result%20Structure%20%28by%20ref%29))
  (bind _asbp_kibby (Utilities|Casting|CastToBP_Kibby OtherActor))
  (bind _returnvalue (Actor|GetActorOfClass "/Game/Dynamic/Animals/Sheep/AutoSpline.AutoSpline_C"))
  (Utilities|IsValid _returnvalue
    (:Is%20Valid
      (if (Variables|/Game/Dynamic/Animals/Sheep/AutoSpline.AutoSpline_C|GetSplineMove _returnvalue)
        (Variables|Default|SetMoveable false)
        (Default|Reverse _returnvalue)
        (Utilities|FlowControl|Delay 1.5)
        (Variables|Default|SetMoveable true)))))

(event OnSeePawn(PawnSensing)
  (params (Pawn :type Pawn%20Object%20Reference))
  (bind _blackboard (Variables|Default|GetBlackboard))
  ;[1 1 1] Gets and sets values for each food
  (bind _returnvalue (Utilities|GetDataTableRow "/Game/Dynamic/ItemMechanic/Fruit.Fruit" (Utilities|String|StringToName (Utilities|GetClassDisplayName (Utilities|GetClass Pawn))))
    (:then
      (Variables|Default|SetOut%20Row%20Timeto%20Eat (.timetoeat _returnvalue))
      (AI|Components|Blackboard|SetValueasFloat _blackboard (Variables|Default|GetTimeToEat) (.timetoeat _returnvalue))
      (AI|Components|Blackboard|SetValueasBool _blackboard (Variables|Default|GetSpotted?) true)
      (Variables|Default|SetMoveable true)
      (Variables|Default|SetLocation (Transformation|GetActorLocation Pawn))
      (Utilities|Array|Add (Variables|Actor|GetTags) (Variables|Default|GetMoveTag))
      (bind _asac_sheep (Utilities|Casting|CastToAC_Sheep (Pawn|GetController)))
      (Default|Spotted _asac_sheep))))

(event OnComponentEndOverlap(KibbySensor)
  (params (OverlappedComponent :type Primitive%20Component%20Object%20Reference) (OtherActor :type Actor%20Object%20Reference) (OtherComp :type Primitive%20Component%20Object%20Reference) (OtherBodyIndex :type Integer))
  (if (Variables|Default|GetMoveable)
    _
    (else
      (Utilities|FlowControl|Delay 0.75)))
  (Utilities|Casting|CastToBP_Kibby OtherActor)
  (bind _returnvalue (Actor|GetActorOfClass "/Game/Dynamic/Animals/Sheep/AutoSpline.AutoSpline_C"))
  (Utilities|IsValid _returnvalue
    (:Is%20Valid
      (Default|Continue _returnvalue))))

(event EventBeginPlay
  (if (Variables|Default|GetMoveable)
    (Utilities|Array|Add (Variables|Actor|GetTags) (Variables|Default|GetMoveTag)))
  (bind _returnvalue (AddComponent|AddBlackboardComponent))
  (Variables|Default|SetBlackboard _returnvalue)
  (Utilities|FlowControl|Delay (Math|Random|RandomFloatinRange 5.0 15.0))
  (switch int (Math|Random|RandomIntegerinRange 0 2)
    (:0
      (Audio|PlaySound2D "/Game/Static/UsedAssets/AudioAssets/SFX/Animal/sheepie_1.sheepie_1" 1.0 1.0 0.0 0 0))
    (:1
      (Audio|PlaySound2D "/Game/Static/UsedAssets/AudioAssets/SFX/Animal/sheepie_2.sheepie_2" 1.0 1.0 0.0 0 0))
    (:2
      (Audio|PlaySound2D "/Game/Static/UsedAssets/AudioAssets/SFX/Animal/sheepie_3.sheepie_3" 1.0 1.0 0.0 0 0))))

(event EventTick
  (params (DeltaSeconds :type Float%20%28single-precision%29))
  ;[1 1 1] Sheep Doesn't Use Hunger So This Is Unused
)

(fn ConstructionScript)

(fn FireSpotted
  (params (Pawn :type Pawn%20Object%20Reference) (Blackboard :type Blackboard%20Component%20Object%20Reference))
  (bind _returnvalue (Transformation|GetActorLocation Pawn))
  (bind _returnvalue_2 (Transformation|GetActorLocation Pawn))
  (bind _returnvalue_3 (Math|Rotator|FindLookatRotation _returnvalue_2 _returnvalue))
  (AI|Components|Blackboard|SetValueasBool Blackboard (Variables|Default|GetFire) true)
  (if (>= (.yaw _returnvalue_3) 0.0)
    (Variables|Default|SetRotation (Math|Rotator|MakeRotator (.roll _returnvalue_3) (.pitch _returnvalue_3) (- (.yaw _returnvalue_3) 1.8e+02)))
    (else
      (Variables|Default|SetRotation (Math|Rotator|MakeRotator (.roll _returnvalue_3) (.pitch _returnvalue_3) (+ (.yaw _returnvalue_3) 1.8e+02)))))
  (Transformation|SetActorRotation (Variables|Default|GetRotation))
  (Class|BlackboardComponent|SetValueasRotator Blackboard (Variables|Default|GetRunAwayDirection) (Variables|Default|GetRotation)))