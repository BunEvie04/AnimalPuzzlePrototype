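; AI controller for the sheep animal that runs its behavior tree.
; It casts the controlled pawn to BP_Sheep and copies its Moveable flag and Location into the Movable and Spot blackboard keys.
; BeginPlay and Tick share this chain, so the tree run call and both blackboard writes repeat every frame.
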(event EventBeginPlay
  (bind _returnvalue (AI|GetBlackboard 0))
  (AI|RunBehaviorTree (Variables|Default|GetBTAsset))
  (bind _asbp_sheep (Utilities|Casting|CastToBP_Sheep (Pawn|GetControlledPawn)))
  (AI|Components|Blackboard|SetValueasBool _returnvalue (Variables|Default|GetMovable) (Variables|/Game/Dynamic/Animals/Sheep/BP_Sheep.BP_Sheep_C|GetMoveable _asbp_sheep))
  (AI|Components|Blackboard|SetValueasVector _returnvalue (Variables|Default|GetSpot) (Variables|/Game/Dynamic/Animals/Sheep/BP_Sheep.BP_Sheep_C|GetLocation _asbp_sheep)))

(event EventTick
  (params (DeltaSeconds :type Float%20%28single-precision%29))
  (bind _returnvalue (AI|GetBlackboard 0))
  (AI|RunBehaviorTree (Variables|Default|GetBTAsset))
  (bind _asbp_sheep (Utilities|Casting|CastToBP_Sheep (Pawn|GetControlledPawn)))
  (AI|Components|Blackboard|SetValueasBool _returnvalue (Variables|Default|GetMovable) (Variables|/Game/Dynamic/Animals/Sheep/BP_Sheep.BP_Sheep_C|GetMoveable _asbp_sheep))
  (AI|Components|Blackboard|SetValueasVector _returnvalue (Variables|Default|GetSpot) (Variables|/Game/Dynamic/Animals/Sheep/BP_Sheep.BP_Sheep_C|GetLocation _asbp_sheep)))

(fn ConstructionScript)