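; BP_Flying is a flying animal that chases the third-person character while it is inside the actor's detection box.
; BeginPlay saves the home location and spawns a separate actor, stored as CollisionBox but not used afterward.
; Box overlaps toggle PlayerDetect, which Tick reads to drive or stop MoveComponentTo toward the player, timed by distance over MoveSpeed.
; A second move returns it home if detection is off when the chase move completes.
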(event OnComponentBeginOverlap(Box)
  (params (OverlappedComponent :type Primitive%20Component%20Object%20Reference) (OtherActor :type Actor%20Object%20Reference) (OtherComp :type Primitive%20Component%20Object%20Reference) (OtherBodyIndex :type Integer) (bFromSweep :type Boolean) (SweepResult :type Hit%20Result%20Structure%20%28by%20ref%29))
  (Utilities|Casting|CastToBP_ThirdPersonCharacter OtherActor)
  (Variables|Default|SetPlayerDetect true))

(event OnComponentEndOverlap(Box)
  (params (OverlappedComponent :type Primitive%20Component%20Object%20Reference) (OtherActor :type Actor%20Object%20Reference) (OtherComp :type Primitive%20Component%20Object%20Reference) (OtherBodyIndex :type Integer))
  (Utilities|Casting|CastToBP_ThirdPersonCharacter OtherActor)
  (Variables|Default|SetPlayerDetect false))

(event Custom|Check)

(event EventBeginPlay
  (Variables|Default|SetDefaultLocation (Transformation|GetActorLocation))
  (bind _returnvalue (Game|SpawnActorfromClass (Variables|Default|GetClass) (Variables|Default|GetSpawn%20Transform) "Undefined" "MultiplyWithRoot" 0 0))
  (Variables|Default|SetCollisionBox _returnvalue))

(event EventTick
  (params (DeltaSeconds :type Float%20%28single-precision%29))
  (bind (_distanceto _distancefrom) (CallFunction|TimingMovement))
  (if (Variables|Default|GetPlayerDetect)
    (bind _returnvalue (Actor|GetActorOfClass "/Game/Dynamic/ThirdPerson/Blueprints/BP_ThirdPersonCharacter.BP_ThirdPersonCharacter_C"))
    (Variables|Default|SetFinalLocation (Transformation|GetActorLocation _returnvalue))
    (Components|MoveComponentTo (Variables|Collision|GetCapsuleComponent) (Variables|Default|GetFinalLocation) "0, 0, 0" false false _distanceto false :!label _label)
    (if (Variables|Default|GetPlayerDetect)
      (goto _label_2 Stop)
      (else
        (Components|MoveComponentTo (Variables|Collision|GetCapsuleComponent) (Variables|Default|GetDefaultLocation) "0, 0, 0" false false _distancefrom false :!label _label_2)))
    (else
      (goto _label Stop))))

(fn ConstructionScript)

(fn TimingMovement
  (bind _returnvalue (Transformation|GetActorLocation))
  (bind _movespeed (Variables|Default|GetMoveSpeed))
  (return (/ (Math|Vector|Distance(Vector) _returnvalue (Variables|Default|GetFinalLocation)) _movespeed) (/ (Math|Vector|Distance(Vector) _returnvalue (Variables|Default|GetDefaultLocation)) _movespeed)))