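; AI controller for Kibby, an animal character driven by a behavior tree.
; It runs the tree, casts the controlled pawn to BP_Kibby and copies its Moveable flag and AppleSpot location into the blackboard's Movable and Spot keys.
; Tick re-enters the BeginPlay chain, so both the RunBehaviorTree call and the blackboard writes repeat every frame.
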(event EventBeginPlay
  (bind _returnvalue (AI|GetBlackboard 0))
  (AI|RunBehaviorTree (Variables|Default|GetBTAsset))
  (bind _asbp_kibby (Utilities|Casting|CastToBP_Kibby (Pawn|GetControlledPawn)))
  (AI|Components|Blackboard|SetValueasBool _returnvalue (Variables|Default|GetMovable) (Variables|/Game/Dynamic/Animals/Kibby/BP_Kibby.BP_Kibby_C|GetMoveable _asbp_kibby))
  (AI|Components|Blackboard|SetValueasVector _returnvalue (Variables|Default|GetSpot) (Variables|/Game/Dynamic/Animals/Kibby/BP_Kibby.BP_Kibby_C|GetAppleSpot _asbp_kibby)))

(event EventTick
  (params (DeltaSeconds :type Float%20%28single-precision%29))
  (bind _returnvalue (AI|GetBlackboard 0))
  (AI|RunBehaviorTree (Variables|Default|GetBTAsset))
  (bind _asbp_kibby (Utilities|Casting|CastToBP_Kibby (Pawn|GetControlledPawn)))
  (AI|Components|Blackboard|SetValueasBool _returnvalue (Variables|Default|GetMovable) (Variables|/Game/Dynamic/Animals/Kibby/BP_Kibby.BP_Kibby_C|GetMoveable _asbp_kibby))
  (AI|Components|Blackboard|SetValueasVector _returnvalue (Variables|Default|GetSpot) (Variables|/Game/Dynamic/Animals/Kibby/BP_Kibby.BP_Kibby_C|GetAppleSpot _asbp_kibby)))

(fn ConstructionScript)