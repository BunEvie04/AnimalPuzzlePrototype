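; Kibby is an AI animal pawn that notices food, gets hungry and flees from fire, feeding its state into a Blackboard.
; Pawn sensing matches seen pawns against the Fruit data table, writes the target and eat time, and makes Kibby moveable.
; While moveable, Tick lowers hunger in the Blackboard and on a camera-facing widget bar.
; Fire entering the detection volume turns Kibby 180 degrees away and stores that escape rotation.
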(event OnComponentBeginOverlap(Detection)
  (params (OverlappedComponent :type Primitive%20Component%20Object%20Reference) (OtherActor :type Actor%20Object%20Reference) (OtherComp :type Primitive%20Component%20Object%20Reference) (OtherBodyIndex :type Integer) (bFromSweep :type Boolean) (SweepResult :type Hit%20Result%20Structure%20%28by%20ref%29))
  (bind _asbp_fire (Utilities|Casting|CastToBP_Fire OtherActor))
  (CallFunction|FireSpotted _asbp_fire (Variables|Default|GetBlackboard)))

(event OnSeePawn(PawnSensing)
  (params (Pawn :type Pawn%20Object%20Reference))
  (bind _blackboard (Variables|Default|GetBlackboard))
  ;[1 1 1] Gets and sets values for each food
  (bind _returnvalue (Utilities|GetDataTableRow "/Game/Dynamic/ItemMechanic/Fruit.Fruit" (Utilities|String|StringToName (Utilities|GetClassDisplayName (Utilities|GetClass Pawn))))
    (:then
      (AI|Components|Blackboard|SetValueasFloat _blackboard (Variables|Keys|GetEattime) (.timetoeat _returnvalue))
      (AI|Components|Blackboard|SetValueasBool _blackboard (Variables|Keys|GetKSpotted) true)
      (AI|Components|Blackboard|SetValueasObject _blackboard (Variables|Default|GetActorNoticed) Pawn)
      (Variables|Default|SetMoveable true)
      (Variables|Default|SetAppleSpot (Transformation|GetActorLocation Pawn))
      (Utilities|Array|Add (Variables|Actor|GetTags) (Variables|Default|GetMoveTag)))
    (:RowNotFound
      (Development|PrintString "Not correct object"))))

(event OnComponentEndOverlap(Detection)
  (params (OverlappedComponent :type Primitive%20Component%20Object%20Reference) (OtherActor :type Actor%20Object%20Reference) (OtherComp :type Primitive%20Component%20Object%20Reference) (OtherBodyIndex :type Integer))
  (Utilities|Casting|CastToBP_Fire OtherActor))

(event EventBeginPlay
  (if (Variables|Default|GetMoveable)
    (Utilities|Array|Add (Variables|Actor|GetTags) (Variables|Default|GetMoveTag)))
  (bind _returnvalue (AddComponent|AddBlackboardComponent))
  (Variables|Default|SetBlackboard _returnvalue)
  (bind _ashungerbar (Utilities|Casting|CastToHungerbar (UserInterface|GetUserWidgetObject (Variables|Default|GetWHunger))))
  (Variables|Default|SetAs%20Hungerbar _ashungerbar))

(event EventTick
  (params (DeltaSeconds :type Float%20%28single-precision%29))
  (bind _blackboard (Variables|Default|GetBlackboard))
  (bind _khunger (Variables|Keys|GetKHunger))
  (bind _returnvalue (Class|BlackboardComponent|GetValueasFloat _blackboard _khunger))
  (bind _returnvalue_2 (- _returnvalue 0.0005))
  (bind _returnvalue_3 (Math|Float|Clamp(Float) _returnvalue_2))
  (CallFunction|UpdateHunger)
  (if (Variables|Default|GetMoveable)
    (AI|Components|Blackboard|SetValueasFloat _blackboard _khunger _returnvalue_3)
    (Variables|/Game/Dynamic/BasicElements/Widgets/Hungerbar.Hungerbar_C|SetCurrentHunger (Variables|Default|GetAs%20Hungerbar) _returnvalue_3)))

(fn ConstructionScript)

(fn UpdateHunger
  (Transformation|SetRelativeRotation (Variables|Default|GetWHunger) (Math|Rotator|FindLookatRotation (Transformation|GetWorldLocation (Variables|Default|GetWHunger)) (Camera|GetCameraLocation (Game|GetPlayerCameraManager 0))) false false)
  (return))

(fn FireSpotted
  (params (Pawn :type Pawn%20Object%20Reference) (Blackboard :type Blackboard%20Component%20Object%20Reference))
  (bind _returnvalue (Transformation|GetActorLocation Pawn))
  (bind _returnvalue_2 (Transformation|GetActorLocation))
  (bind _returnvalue_3 (Math|Rotator|FindLookatRotation _returnvalue_2 _returnvalue))
  (AI|Components|Blackboard|SetValueasBool Blackboard (Variables|Keys|GetFire) true)
  (if (>= (.yaw _returnvalue_3) 0.0)
    (Variables|Default|SetRotation (Math|Rotator|MakeRotator (.roll _returnvalue_3) (.pitch _returnvalue_3) (- (.yaw _returnvalue_3) 1.8e+02)))
    (else
      (Variables|Default|SetRotation (Math|Rotator|MakeRotator (.roll _returnvalue_3) (.pitch _returnvalue_3) (+ (.yaw _returnvalue_3) 1.8e+02)))))
  (Transformation|SetActorRotation (Variables|Default|GetRotation))
  (Class|BlackboardComponent|SetValueasRotator Blackboard (Variables|Keys|GetRunAwayDirection) (Variables|Default|GetRotation)))