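; BP_Kibby is an animal Blueprint that uses pawn sensing to spot apples.
; It adds a Blackboard component on BeginPlay.
; When the sensed pawn's class is exactly BP_Apples, it sets the KSpotted blackboard key, flags itself as moveable and stores the apple's location; other pawns only print a debug message.
; An unconnected debug line trace is left in the graph.
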(event OnSeePawn(PawnSensing)
  (params (Pawn :type Pawn%20Object%20Reference))
  (if (== (Utilities|GetClass Pawn) "/Game/Dynamic/ItemMechanic/Fruits/BP_Apples.BP_Apples_C")
    (AI|Components|Blackboard|SetValueasBool (stale EventBeginPlay _returnvalue) (Variables|Default|GetKSpotted) true)
    (Variables|Default|SetMoveable true)
    (Variables|Default|SetAppleSpot (Transformation|GetActorLocation Pawn))
    (else
      (Development|PrintString "Not correct object"))))

(event EventBeginPlay
  (bind _returnvalue (AddComponent|AddBlackboardComponent))
  (Variables|Default|SetBlackboard _returnvalue))

(event Collision|EventActorBeginOverlap
  (params (OtherActor :type Actor%20Object%20Reference)))

(event EventTick
  (params (DeltaSeconds :type Float%20%28single-precision%29)))

(fn ConstructionScript)