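; AI controller for the cat animal that runs its behavior tree and feeds it state from the controlled BP_Cat pawn.
; It copies the cat's Moveable flag and AppleSpot location into the Movable and Spot blackboard keys.
; BeginPlay and Tick share the same chain, so RunBehaviorTree is called again every frame along with the blackboard update.
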(event EventBeginPlay
  (bind _returnvalue (AI|GetBlackboard 0))
  (AI|RunBehaviorTree (Variables|Default|GetBTAsset))
  (bind _asbp_cat (Utilities|Casting|CastToBP_Cat (Pawn|GetControlledPawn)))
  (AI|Components|Blackboard|SetValueasBool _returnvalue (Variables|Default|GetMovable) (Variables|/Game/Dynamic/Animal2/BP_Cat.BP_Cat_C|GetMoveable _asbp_cat))
  (AI|Components|Blackboard|SetValueasVector _returnvalue (Variables|Default|GetSpot) (Variables|/Game/Dynamic/Animal2/BP_Cat.BP_Cat_C|GetAppleSpot _asbp_cat)))

(event EventTick
  (params (DeltaSeconds :type Float%20%28single-precision%29))
  (bind _returnvalue (AI|GetBlackboard 0))
  (AI|RunBehaviorTree (Variables|Default|GetBTAsset))
  (bind _asbp_cat (Utilities|Casting|CastToBP_Cat (Pawn|GetControlledPawn)))
  (AI|Components|Blackboard|SetValueasBool _returnvalue (Variables|Default|GetMovable) (Variables|/Game/Dynamic/Animal2/BP_Cat.BP_Cat_C|GetMoveable _asbp_cat))
  (AI|Components|Blackboard|SetValueasVector _returnvalue (Variables|Default|GetSpot) (Variables|/Game/Dynamic/Animal2/BP_Cat.BP_Cat_C|GetAppleSpot _asbp_cat)))

(fn ConstructionScript)