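; BP_Activate1 is a trigger-box activator that changes how BP_Foxling moves inside it, based on a water/rain enum.
; Slight Water slows the foxling, while Heavy Rain clears its Stationary flag and calls Stationary on its AC_Animal controller.
; Both cases show the foxling's Cube and make it block pawns; leaving hides it, ignores pawns and restores movement.
; BeginPlay sets Playable only for Heavy Rain.
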(event OnComponentBeginOverlap(Box)
  (params (OverlappedComponent :type Primitive%20Component%20Object%20Reference) (OtherActor :type Actor%20Object%20Reference) (OtherComp :type Primitive%20Component%20Object%20Reference) (OtherBodyIndex :type Integer) (bFromSweep :type Boolean) (SweepResult :type Hit%20Result%20Structure%20%28by%20ref%29))
  (bind _asbp_foxling (Utilities|Casting|CastToBP_Foxling OtherActor))
  (switch Utilities|FlowControl|Switch|SwitchonEnum_Lvl1Act (Variables|Default|GetEnum)
    (:NewEnumerator0
      (Default|SlowedMovement _asbp_foxling))
    (:NewEnumerator1
      (Variables|/Game/Dynamic/Animals/Foxling/BP_Foxling.BP_Foxling_C|Set!Stationary _asbp_foxling false)
      (bind _asac_animal (Utilities|Casting|CastToAC_Animal (AI|GetAIController _asbp_foxling)))
      (Default|Stationary _asac_animal)))
  (Rendering|SetVisibility (Variables|/Game/Dynamic/Animals/Foxling/BP_Foxling.BP_Foxling_C|GetCube _asbp_foxling) true false)
  (Collision|SetCollisionResponsetoChannel (Variables|/Game/Dynamic/Animals/Foxling/BP_Foxling.BP_Foxling_C|GetCube _asbp_foxling) "ECC_Pawn" "ECR_Block"))

(event OnComponentEndOverlap(Box)
  (params (OverlappedComponent :type Primitive%20Component%20Object%20Reference) (OtherActor :type Actor%20Object%20Reference) (OtherComp :type Primitive%20Component%20Object%20Reference) (OtherBodyIndex :type Integer))
  (bind _asbp_foxling (Utilities|Casting|CastToBP_Foxling OtherActor))
  (Rendering|SetVisibility (Variables|/Game/Dynamic/Animals/Foxling/BP_Foxling.BP_Foxling_C|GetCube _asbp_foxling) false false)
  (Collision|SetCollisionResponsetoChannel (Variables|/Game/Dynamic/Animals/Foxling/BP_Foxling.BP_Foxling_C|GetCube _asbp_foxling) "ECC_Pawn" "ECR_Ignore")
  (Default|RestoreMovement _asbp_foxling))

(event EventBeginPlay
  (if (Utilities|Enum|Equal(Enum) (Variables|Default|GetEnum) "NewEnumerator1")
    (Variables|Default|SetPlayable true)
    (else
      (Variables|Default|SetPlayable false))))

(fn ConstructionScript)