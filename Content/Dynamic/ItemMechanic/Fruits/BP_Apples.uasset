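; BP_Apples is a fruit item actor that a spawner grows and animals eat.
; Growth and Eaten play timelines that lerp actor scale, growing it from small to full size or shrinking it to zero before destroying it.
; LookAt returns the item's display name from the data table row referenced by its ItemDataComp.
; The collision overlap event is empty.
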(event OnComponentBeginOverlap(Collision)
  (params (OverlappedComponent :type Primitive%20Component%20Object%20Reference) (OtherActor :type Actor%20Object%20Reference) (OtherComp :type Primitive%20Component%20Object%20Reference) (OtherBodyIndex :type Integer) (bFromSweep :type Boolean) (SweepResult :type Hit%20Result%20Structure%20%28by%20ref%29)))

(event Custom|Growth
  ;[0.2708 0.2708 0.2708] Called by Spawner, Grows Actor
  (bind _simple1_0 (Timeline|Timeline Play)
    (:Update
      (Transformation|SetActorScale3D (Math|Vector|Lerp(Vector) "0.100000,0.100000,0.100000" "1.000000,1.000000,1.000000" _simple1_0)))))

(event Custom|Eaten
  ;[1 1 1] Called by Animal, Destroy Actor
  (bind _simple0_1 (Timeline|ShrinkLine Play)
    (:Update
      (Transformation|SetActorScale3D (Math|Vector|Lerp(Vector) "1.000000,1.000000,1.000000" "0, 0, 0" _simple0_1)))
    (:Finished
      (Actor|DestroyActor))))

(fn ConstructionScript)

(fn Lookat
  (bind _itemdatacomp (Variables|Default|GetItemDataComp))
  (bind _itemid (Variables|/Game/Dynamic/ItemMechanic/Inventory/ItemDataComp.ItemDataComp_C|GetItemID _itemdatacomp))
  (bind _returnvalue (Utilities|GetDataTableRow (.datatable _itemid) (.rowname _itemid))
    (:then
      (return (Utilities|Text|FormatText (.Name (Utilities|Struct|BreakFList _returnvalue)))))))