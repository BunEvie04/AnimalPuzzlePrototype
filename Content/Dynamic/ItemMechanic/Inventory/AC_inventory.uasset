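; AC_inventory is an inventory actor component that currently handles look-at detection for interaction, with adding and removing items left as empty stubs.
; Every tick it runs a sphere trace on the Visibility channel from the player camera along its forward vector up to the interact range, ignoring the owner.
; A hit actor is stored as LookAt and its LookAtMessage is printed, while a miss clears LookAt.
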(event EventTick
  (params (DeltaSeconds :type Float%20%28single-precision%29))
  (CallFunction|InteractionTrace))

(event EventBeginPlay)

(event Input|KeyboardEvents|E
  (params (Key :type Key%20Structure :default "None")))

(fn AddtoInventory)

(fn RemovefromInventory)

(fn InteractionTrace
  (bind _returnvalue (Game|GetPlayerCameraManager 0))
  (bind _returnvalue_2 (Transformation|GetActorLocation _returnvalue))
  (bind (_outhit _returnvalue_3) (Collision|SphereTraceByChannel _returnvalue_2 (+ _returnvalue_2 (* (Transformation|GetActorForwardVector _returnvalue) (Variables|Default|GetIneractRange))) 0.0 "TraceTypeQuery1" false (Utilities|Array|MakeArray (Components|GetOwner)) "None"))
  (if _returnvalue_3
    (bind _output_get (Variables|Default|SetLookAt (.HitActor (Collision|BreakHitResult _outhit))))
    (bind _lookat (Class|IntTimeline|Lookat(Message) _output_get))
    (Development|PrintText _lookat)
    (else
      (Variables|Default|SetLookAt 0))))