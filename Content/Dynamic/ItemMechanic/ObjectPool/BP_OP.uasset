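; Object pool actor that pre-spawns and recycles actors of one class for an item ID.
; InitialisePool reads class and amount from the DT_OP row, then spawns that many hidden, collision-disabled actors into PooledObjects.
; RemovefromPool reactivates and returns the first hidden entry, without growing the pool, while AddtoPool deactivates and stores an actor again.
; The InitialisePool call in the event graph is unwired, so BeginPlay leaves the pool empty.
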(event EventBeginPlay)

(event Collision|EventActorBeginOverlap
  (params (OtherActor :type Actor%20Object%20Reference)))

(event EventTick
  (params (DeltaSeconds :type Float%20%28single-precision%29)))

(fn ConstructionScript)

(fn InitialisePool
  (bind _returnvalue (Utilities|GetDataTableRow "/Game/Dynamic/ItemMechanic/ObjectPool/DT_OP.DT_OP" (Variables|Default|GetItemID))
    (:then
      (bind _output_get (Variables|Default|SetObjectClass (.class _returnvalue)))
      (bind _output_get_2 (Variables|Default|SetPoolSize (.amount _returnvalue)))
      (for _index (range 0 (- _output_get_2 1))
        (bind _returnvalue_2 (Game|SpawnActorfromClass _output_get (Transformation|GetActorTransform) "Undefined" "MultiplyWithRoot" 0 0))
        (Rendering|SetActorHiddenInGame _returnvalue_2 true)
        (Collision|SetActorEnableCollision _returnvalue_2 false)
        (Utilities|Array|Add (Variables|Default|GetPooledObjects) _returnvalue_2)))))

(fn RemovefromPool
  (for _array_element (Variables|Default|GetPooledObjects)
    (if (Variables|/Script/Engine.Actor|GetbHidden _array_element)
      (Rendering|SetActorHiddenInGame _array_element false)
      (Collision|SetActorEnableCollision _array_element true)
      (Utilities|Array|RemoveItem (Variables|Default|GetPooledObjects) _array_element)
      (return _array_element))))

(fn AddtoPool
  (params (PooledObject :type Actor%20Object%20Reference))
  (Rendering|SetActorHiddenInGame PooledObject true)
  (Collision|SetActorEnableCollision PooledObject false)
  (Utilities|Array|Add (Variables|Default|GetPooledObjects) PooledObject))