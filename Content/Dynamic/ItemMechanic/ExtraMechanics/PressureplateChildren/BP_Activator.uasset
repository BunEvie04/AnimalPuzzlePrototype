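; Pressure-plate activator that toggles a FinalSpot component and spawns a BP_CageBase at its location.
; An overlap by an actor with the SelectedActivator tag either hides a visible spot and spawns a scaled cage, or shows the hidden spot with collision.
; If State is set, the cage spawns at BeginPlay.
; A third-person character entering the Box sets MainSpawn, then releases and destroys the spawned cage.
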(event OnComponentBeginOverlap(Box)
  (params (OverlappedComponent :type Primitive%20Component%20Object%20Reference) (OtherActor :type Actor%20Object%20Reference) (OtherComp :type Primitive%20Component%20Object%20Reference) (OtherBodyIndex :type Integer) (bFromSweep :type Boolean) (SweepResult :type Hit%20Result%20Structure%20%28by%20ref%29))
  (Utilities|Casting|CastToBP_ThirdPersonCharacter OtherActor)
  (Variables|Default|SetMainSpawn true)
  (Default|Release (Variables|Default|GetSpawned%20Cage))
  (Actor|DestroyActor (Variables|Default|GetSpawned%20Cage)))

(event Custom|ActivatedComponent
  (bind _finalspot (Variables|Default|GetFinalSpot))
  (if (Variables|/Script/Engine.SceneComponent|GetbVisible _finalspot)
    (CallFunction|SpawnObject)
    (else
      (Development|PrintString "no")
      (Rendering|SetVisibility _finalspot true false)
      (Collision|SetCollisionEnabled _finalspot "QueryAndPhysics"))))

(event Custom|MainMove)

(event EventBeginPlay
  (Variables|Default|SetMainSpawn false)
  (Variables|Default|SetActivateLocation (Transformation|GetWorldLocation (Variables|Default|GetFinalSpot)))
  (if (Variables|Default|GetState)
    (CallFunction|SpawnObject)))

(event Collision|EventActorBeginOverlap
  (params (OtherActor :type Actor%20Object%20Reference))
  ;[1 1 1] Detects player
  (if (Actor|ActorHasTag OtherActor (Variables|Default|GetSelectedActivator))
    (CallFunction|ActivatedComponent)))

(fn ConstructionScript)

(fn SpawnObject
  (bind _returnvalue (Transformation|GetActorScale3D))
  (bind _finalspot (Variables|Default|GetFinalSpot))
  (Rendering|SetVisibility _finalspot false false)
  (Collision|SetCollisionEnabled _finalspot "NoCollision")
  (bind _returnvalue_2 (Game|SpawnActorfromClass "/Game/Dynamic/ItemMechanic/ExtraMechanics/BP_CageBase.BP_CageBase_C" (Math|Transform|MakeTransform (Variables|Default|GetActivateLocation) (Transformation|GetActorRotation) (Math|Vector|MakeVector (* (.x _returnvalue) 1.85) (* (.y _returnvalue) 1.85) (* (.z _returnvalue) 1.75))) "Undefined" "MultiplyWithRoot" 0 0))
  (Variables|Default|SetSpawned%20Cage _returnvalue_2)
  (Development|PrintString "Hello"))