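; BP_Count is a pressure plate counter that ends the level with a win screen once enough sheep reach it.
; Each BP_Sheep overlap on ButtonCollision is appended to an array, and returned index 3, the fourth entry, triggers the win.
; The win widget shows for three seconds before the Title level opens.
; Entries are never removed or deduplicated, and the parent-plate lookup and MaxCount check are unconnected.
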(event OnComponentBeginOverlap(ButtonCollision)
  (params (OverlappedComponent :type Primitive%20Component%20Object%20Reference) (OtherActor :type Actor%20Object%20Reference) (OtherComp :type Primitive%20Component%20Object%20Reference) (OtherBodyIndex :type Integer) (bFromSweep :type Boolean) (SweepResult :type Hit%20Result%20Structure%20%28by%20ref%29))
  (bind _asbp_sheep (Utilities|Casting|CastToBP_Sheep OtherActor))
  (bind _returnvalue (Utilities|Array|Add (Variables|Default|GetArr) _asbp_sheep))
  (if (== _returnvalue 3)
    (bind _returnvalue_2 (UserInterface|CreateWidget "/Game/Dynamic/BasicElements/Widgets/WP_WinScr.WP_WinScr_C"))
    (bind _output_get (Variables|Default|SetNewVar _returnvalue_2))
    (UserInterface|Viewport|AddtoViewport _output_get 0)
    (Utilities|FlowControl|Delay 3.0)
    (Game|OpenLevel(byName) "Title")
    (Widget|RemovefromParent _output_get)))

(event EventBeginPlay
  ;[1 1 1] Gets the array of actors on top
)

(event Collision|EventActorBeginOverlap
  (params (OtherActor :type Actor%20Object%20Reference))
  ;[1 1 1] Sets Result Based on No of Actors
)

(fn ConstructionScript)