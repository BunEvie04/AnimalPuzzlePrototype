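; BP_CageBase is a cage actor with a physics part, CagePart2, whose movement axes depend on where the player stands.
; When BP_ThirdPersonCharacter overlaps GrabBack or GrabLeft, CagePart2's constraint mode becomes the XZ or YZ plane respectively.
; Ending an overlap on either volume restores the default mode, and Tick keeps the actor's rotation at zero.
; Caged overlap and Release events are empty, leaving the BP_Sheep capture and release logic disconnected.
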(event OnComponentBeginOverlap(GrabLeft)
  (params (OverlappedComponent :type Primitive%20Component%20Object%20Reference) (OtherActor :type Actor%20Object%20Reference) (OtherComp :type Primitive%20Component%20Object%20Reference) (OtherBodyIndex :type Integer) (bFromSweep :type Boolean) (SweepResult :type Hit%20Result%20Structure%20%28by%20ref%29))
  ;[1 1 1] Enables movement on axis
  (Utilities|Casting|CastToBP_ThirdPersonCharacter OtherActor)
  (Class|PrimitiveComponent|SetConstraintMode (Variables|Default|GetCagePart2) "YZPlane"))

(event OnComponentEndOverlap(GrabLeft)
  (params (OverlappedComponent :type Primitive%20Component%20Object%20Reference) (OtherActor :type Actor%20Object%20Reference) (OtherComp :type Primitive%20Component%20Object%20Reference) (OtherBodyIndex :type Integer))
  ;[1 1 1] Disables Movement
  (Class|PrimitiveComponent|SetConstraintMode (Variables|Default|GetCagePart2) "Default"))

(event OnComponentBeginOverlap(GrabBack)
  (params (OverlappedComponent :type Primitive%20Component%20Object%20Reference) (OtherActor :type Actor%20Object%20Reference) (OtherComp :type Primitive%20Component%20Object%20Reference) (OtherBodyIndex :type Integer) (bFromSweep :type Boolean) (SweepResult :type Hit%20Result%20Structure%20%28by%20ref%29))
  ;[1 1 1] Enables movement on axis
  (Utilities|Casting|CastToBP_ThirdPersonCharacter OtherActor)
  (Class|PrimitiveComponent|SetConstraintMode (Variables|Default|GetCagePart2) "XZPlane"))

(event OnComponentEndOverlap(GrabBack)
  (params (OverlappedComponent :type Primitive%20Component%20Object%20Reference) (OtherActor :type Actor%20Object%20Reference) (OtherComp :type Primitive%20Component%20Object%20Reference) (OtherBodyIndex :type Integer))
  ;[1 1 1] Disables Movement
  (Class|PrimitiveComponent|SetConstraintMode (Variables|Default|GetCagePart2) "Default"))

(event OnComponentBeginOverlap(Caged)
  (params (OverlappedComponent :type Primitive%20Component%20Object%20Reference) (OtherActor :type Actor%20Object%20Reference) (OtherComp :type Primitive%20Component%20Object%20Reference) (OtherBodyIndex :type Integer) (bFromSweep :type Boolean) (SweepResult :type Hit%20Result%20Structure%20%28by%20ref%29)))

(event OnComponentEndOverlap(Caged)
  (params (OverlappedComponent :type Primitive%20Component%20Object%20Reference) (OtherActor :type Actor%20Object%20Reference) (OtherComp :type Primitive%20Component%20Object%20Reference) (OtherBodyIndex :type Integer)))

(event Custom|Release)

(event EventTick
  (params (DeltaSeconds :type Float%20%28single-precision%29))
  (Transformation|SetActorRotation "0, 0, 0"))

(fn ConstructionScript)